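; GameUI_GM is a game mode Blueprint that runs the startup logo sequence and then opens the main menu UI.
; On BeginPlay it plays a startup sound and shows an animated logo widget with the cursor hidden and UI-only input.
; After a fixed delay it starts ambient UI audio, adds the animated MainUI widget and shows the cursor.
; The logo widget is never explicitly removed here.
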(event `self.ReceiveBeginPlay`
  (bind _returnvalue (`GameplayStatics.GetPlayerController` 0))
  (bind _returnvalue_2 (`GameplayStatics.GetPlayerController` 0))
  (`GameplayStatics.PlaySound2D` "/Game/UI/UISFX/GameStartupSound.GameStartupSound" 1.0 1.0 0.0 null null)
  (bind _returnvalue_3 (`|CreateWidget` "/Game/UI/LogoScreen.LogoScreen_C"))
  (`UserWidget.PlayAnimation` _returnvalue_3 (`/Game/UI/LogoScreen.AppearDisappear` _returnvalue_3) 0.0 1 "Forward" 1.0 false)
  (`UserWidget.AddToViewport` _returnvalue_3 0)
  (set `PlayerController.bShowMouseCursor` false _returnvalue_2)
  (`WidgetBlueprintLibrary.SetInputMode_UIOnlyEx` _returnvalue_2 _returnvalue_3)
  (`KismetSystemLibrary.Delay` 10.0)
  (`GameplayStatics.PlaySound2D` "/Game/UI/UISFX/AmbientUI.AmbientUI" 1.0 1.0 0.0 null null)
  (bind _returnvalue_4 (`|CreateWidget` "/Game/UI/MainUI.MainUI_C"))
  (`UserWidget.PlayAnimation` _returnvalue_4 (`/Game/UI/MainUI.Appear` _returnvalue_4) 0.0 1 "Forward" 1.0 false)
  (`UserWidget.AddToViewport` _returnvalue_4 0)
  (set `PlayerController.bShowMouseCursor` true _returnvalue)
  (`WidgetBlueprintLibrary.SetInputMode_UIOnlyEx` _returnvalue _returnvalue_4))

(fn `UserConstructionScript`)